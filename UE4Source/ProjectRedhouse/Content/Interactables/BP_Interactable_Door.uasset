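; Interactable door Blueprint that plays an opening animation on both the interacting pawn and the door.
; It builds on parent interaction events, overriding MontagePlay to run the player and door montages together.
; After a delay matching the player montage's returned length, it sets Open and calls MontageEnd.
; The Open check has empty branches, so only the prograde opening is implemented, with no closing logic.
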(event `self.ReceiveActorBeginOverlap`
  (params (OtherActor :type "Actor Object Reference"))
  (`parent.ReceiveActorBeginOverlap` OtherActor))

(event `self.Interact`
  (params (Instigator :type "Character Object Reference"))
  (`parent.Interact` Instigator))

(event `self.MontagePlay`
  (`parent.MontagePlay`)
  (if (`self.Open`)
    _
    (else
      _))
  (bind _returnvalue (`AnimInstance.Montage_Play` (`SkeletalMeshComponent.GetAnimInstance` (`Character.Mesh` (`self.InteractingPawn`))) (`self.PlayerOpenPrograde`) 1.0 "MontageLength" 0.0))
  (`AnimInstance.Montage_Play` (`SkeletalMeshComponent.GetAnimInstance` (`self.Door`)) (`self.DoorOpenPrograde`) 1.0 "MontageLength" 0.0)
  (`KismetSystemLibrary.Delay` _returnvalue)
  (set `self.Open` true)
  (`self.MontageEnd`))

(fn `UserConstructionScript`
  (`parent.UserConstructionScript`))