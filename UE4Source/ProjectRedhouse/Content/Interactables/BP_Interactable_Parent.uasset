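; Base interactable actor that moves an ALS player character to an entry point before starting an interaction.
; Interact converts the actor-relative entry transform to world space and, if MatchLocation is set, Tick interpolates the pawn there, compensating for time dilation, while the character matches rotation.
; A timer ends matching and calls MontagePlay, which only sets Activated.
; MontageEnd clears Activated and calls StopInteract on the character.
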(event `self.ReceiveTick`
  (params (DeltaSeconds :type "Float (single-precision)"))
  (if (`self.MatchingLocation`)
    (if (`self.MatchLocation`)
      (bind (_currenttransform _destination _rotation _scale) (`self.CalculateTransform`))
      (`self.K2_SetActorTransform` (`self.InteractingPawn`) (`KismetMathLibrary.TInterpTo` _currenttransform (`KismetMathLibrary.MakeTransform` _destination _rotation _scale) (`GameplayStatics.GetWorldDeltaSeconds`) (/ (/ 2.0 (`GameplayStatics.GetGlobalTimeDilation`)) (`self.MatchLoctionTime`))) false false))))

(fn `CalculateTransform`
  (returns (CurrentTransform :type "Transform Structure") (Destination :type "Vector Structure") (Rotation :type "Rotator Structure") (Scale :type "Vector Structure"))
  (bind _interactingpawn (`self.InteractingPawn`))
  (return (`self.GetTransform` _interactingpawn) (`self.EntryLoc`) (`KismetMathLibrary.MakeRotator` 0.0 0.0 (.yaw (`self.EntryRot`))) (`self.GetActorScale3D` _interactingpawn)))

(fn `Interact`
  (params (Instigator :type "Character Object Reference") (EntryLoc :type "Vector Structure") (EntryRot :type "Rotator Structure") (Time :type "Float (double-precision)"))
  (bind _returnvalue (`self.K2_GetActorRotation`))
  (set `self.MatchLoctionTime` Time)
  (set `self.EntryLoc` (+ (`KismetMathLibrary.GreaterGreater_VectorRotator` EntryLoc _returnvalue) (`self.K2_GetActorLocation`)))
  (set `self.EntryRot` (`KismetMathLibrary.ComposeRotators` EntryRot _returnvalue))
  (bind _output_get (set `self.InteractingPawn` Instigator))
  (set `self.MatchingLocation` true)
  (`/Game/AdvancedLocomotionV2/Blueprints/ALS_Player_CharacterBP.StartInteract` (cast `/Game/AdvancedLocomotionV2/Blueprints/ALS_Player_CharacterBP` _output_get :!pure true))
  (if (`self.MatchLocation`)
    (`self.MatchLoc`)
    (`KismetSystemLibrary.K2_SetTimer` null "MatchLocEnd" (`self.MatchLoctionTime`))
    (else
      (`self.MontagePlay`))))

(fn `MatchLoc`
  (set `self.MatchingLocation` true)
  (bind _asals_player_character_bp (cast `/Game/AdvancedLocomotionV2/Blueprints/ALS_Player_CharacterBP` (`self.InteractingPawn`)))
  (`/Game/AdvancedLocomotionV2/Blueprints/ALS_Player_CharacterBP.MatchRotation` _asals_player_character_bp (`self.EntryRot`) (`self.MatchYaw`)))

(fn `MatchLocEnd`
  (set `self.MatchingLocation` false)
  (bind _asals_player_character_bp (cast `/Game/AdvancedLocomotionV2/Blueprints/ALS_Player_CharacterBP` (`self.InteractingPawn`)))
  (`/Game/AdvancedLocomotionV2/Blueprints/ALS_Player_CharacterBP.MatchRotationEnd` _asals_player_character_bp)
  (`self.MontagePlay`))

(fn `MontageEnd`
  (set `self.Activated` false)
  (bind _asals_player_character_bp (cast `/Game/AdvancedLocomotionV2/Blueprints/ALS_Player_CharacterBP` (`self.InteractingPawn`)))
  (`/Game/AdvancedLocomotionV2/Blueprints/ALS_Player_CharacterBP.StopInteract` _asals_player_character_bp))

(fn `MontagePlay`
  (set `self.Activated` true))

(fn `UserConstructionScript`)